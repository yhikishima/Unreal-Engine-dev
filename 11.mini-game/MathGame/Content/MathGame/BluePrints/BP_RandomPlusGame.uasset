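; Actor Blueprint for a math quiz that shows addition problems with a hidden first operand, answered with number keys 1 to 9.
; BeginPlay enables player input and generates the first problem through RandomCaluculation, which returns two random single-digit operands and their sum.
; Each key sets Answer and joins a shared chain that prints True or False against NumA, then prints a new problem.
; All feedback uses PrintString.
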(event `Key|Six`
  (params (Key :type "Key Structure"))
  ;[1 1 1] キーボード6を入力
  (:`Pressed`
    (set `self.Answer` 6)
    (`KismetSystemLibrary.PrintString` (`KismetStringLibrary.Conv_IntToString` (`self.Answer`)) :!label _label)
    (if (== (`self.NumA`) (`self.Answer`))
      (`KismetSystemLibrary.PrintString` "True")
      (else
        (`KismetSystemLibrary.PrintString` "False")))
    (bind (_localnuma1 _localnumb1 _returnvalue) (`self.RandomCaluculation` :!label _label_2))
    (set `self.NumA` _localnuma1)
    (set `self.NumB` _localnumb1)
    (set `self.Total` _returnvalue)
    (`KismetSystemLibrary.PrintString` (`KismetStringLibrary.Concat_StrStr` "?" "+" (`KismetStringLibrary.Conv_IntToString` (`self.NumB`)) "=" (`KismetStringLibrary.Conv_IntToString` (`self.Total`))) true true (struct :`G` 0.66 :`B` 1.0 :`A` 1.0) (`self.PrintStringDuration`))))

(event `Key|Seven`
  (params (Key :type "Key Structure"))
  ;[1 1 1] キーボード7を入力
  (:`Pressed`
    (set `self.Answer` 7)
    (goto _label)))

(event `Key|Eight`
  (params (Key :type "Key Structure"))
  ;[1 1 1] キーボード8を入力
  (:`Pressed`
    (set `self.Answer` 8)
    (goto _label)))

(event `Key|Nine`
  (params (Key :type "Key Structure"))
  ;[1 1 1] キーボード9を入力
  (:`Pressed`
    (set `self.Answer` 9)
    (goto _label)))

(event `Key|Two`
  (params (Key :type "Key Structure"))
  ;[1 1 1] キーボード2を入力
  (:`Pressed`
    (set `self.Answer` 2)
    (goto _label)))

(event `Key|Three`
  (params (Key :type "Key Structure"))
  ;[1 1 1] キーボード3を入力
  (:`Pressed`
    (set `self.Answer` 3)
    (goto _label)))

(event `Key|Four`
  (params (Key :type "Key Structure"))
  ;[1 1 1] キーボード4を入力
  (:`Pressed`
    (set `self.Answer` 4)
    (goto _label)))

(event `Key|Five`
  (params (Key :type "Key Structure"))
  ;[1 1 1] キーボード5を入力
  (:`Pressed`
    (set `self.Answer` 5)
    (goto _label)))

(event `Key|One`
  (params (Key :type "Key Structure"))
  ;[1 1 1] キーボードを入力
  (:`Pressed`
    (set `self.Answer` 1)
    (goto _label)))

(event `self.ReceiveBeginPlay`
  ;[1 1 1] 入力を受け付ける処理
  (`self.EnableInput` (`GameplayStatics.GetPlayerController` 0))
  (goto _label_2))

(fn `Plus`
  (params (A :type Integer) (B :type Integer) (Tot :type Integer) (NewParam1 :type Boolean))
  (returns (Total :type Integer))
  (return (+ A B)))

(fn `RandomCaluculation`
  (returns (LocalNumA1 :type Integer) (LocalNumB1 :type Integer) (ReturnValue :type Integer))
  (locals (LocalNumA :type Integer) (LocalNumB :type Integer))
  (bind _returnvalue (`KismetMathLibrary.RandomIntegerInRange` 1 9))
  (bind _localnuma (`local.LocalNumA`))
  (bind _localnumb (`local.LocalNumB`))
  ;[1 1 1] ローカル変数にランダム値を格納
  (set `local.LocalNumA` _returnvalue)
  (set `local.LocalNumB` _returnvalue)
  (return _localnuma _localnumb (+ _localnuma _localnumb)))

(fn `UserConstructionScript`)