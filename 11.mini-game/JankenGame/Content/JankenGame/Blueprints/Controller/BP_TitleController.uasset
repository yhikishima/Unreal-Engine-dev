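; Title screen controller for the Janken game that creates the title widget, plays title music and keeps the mouse cursor visible.
; It binds widget events for quitting, starting and changing resolution; starting shows a loading widget, then opens the Game level after a fixed delay.
; Resolution is loaded from and saved through BP_GameInstance, then applied with r.setRes console commands for fullscreen or windowed modes.
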(event `self.ReceiveBeginPlay`
  (bind _asbp_game_instance (cast `/Game/JankenGame/Core/BP_GameInstance` (`GameplayStatics.GetGameInstance`) :!pure true))
  (bind _returnvalue (`|CreateWidget` "/Game/JankenGame/Blueprints/UMG/WBP_Title.WBP_Title_C"))
  (`UserWidget.AddToViewport` _returnvalue 0)
  (add `/Game/JankenGame/Blueprints/UMG/WBP_Title.OnClickedGameExit` _returnvalue (delegate `OnClickedGameExit`))
  (add `/Game/JankenGame/Blueprints/UMG/WBP_Title.OnClickedGameStart` _returnvalue (delegate `OnClickedGameStart`))
  (add `/Game/JankenGame/Blueprints/UMG/WBP_Title.OnSelectionChangedResolution` _returnvalue (delegate `OnSelectionChnagedResolution`))
  (`/Game/JankenGame/Core/BP_GameInstance.LoadGameSettings` _asbp_game_instance)
  (`self.SetResolution` (`/Game/JankenGame/Core/BP_GameInstance.Resolution` _asbp_game_instance))
  (`GameplayStatics.PlaySound2D` "/Game/JankenGame/Audio/BGM/A_Janken_Title_Cue.A_Janken_Title_Cue" 1.0 1.0 0.0 null null))

(event `OnClickedGameExit`
  (`KismetSystemLibrary.QuitGame` null "Quit"))

(event `self.ReceiveTick`
  (params (DeltaSeconds :type "Float (single-precision)"))
  (set `PlayerController.bShowMouseCursor` true (`GameplayStatics.GetPlayerController` 0)))

(event `OnSelectionChnagedResolution`
  (params (Resolution :type "/Game/JankenGame/Blueprints/Enums/EResolution Enum" :default "NewEnumerator0"))
  (bind _asbp_game_instance (cast `/Game/JankenGame/Core/BP_GameInstance` (`GameplayStatics.GetGameInstance`) :!pure true))
  (bind _output_get (set `/Game/JankenGame/Core/BP_GameInstance.Resolution` Resolution _asbp_game_instance))
  (`self.SetResolution` _output_get)
  (`/Game/JankenGame/Core/BP_GameInstance.SaveGameSettings` _asbp_game_instance))

(event `OnClickedGameStart`
  (bind _returnvalue (`|CreateWidget` "/Game/JankenGame/Blueprints/UMG/WBP_Loading.WBP_Loading_C"))
  (`UserWidget.AddToViewport` _returnvalue 0)
  (`KismetSystemLibrary.Delay` 2.0)
  (`GameplayStatics.OpenLevel` "Game"))

(fn `SetResolution`
  (params (Resolution :type "/Game/JankenGame/Blueprints/Enums/EResolution Enum" :default "NewEnumerator0"))
  (returns (ReturnValue :type Boolean))
  (switch `/Game/JankenGame/Blueprints/Enums/EResolution` Resolution
    (:`NewEnumerator0`
      (`KismetSystemLibrary.ExecuteConsoleCommand` "r.setRes 1920x1080f" null))
    (:`NewEnumerator1`
      (`KismetSystemLibrary.ExecuteConsoleCommand` "r.setRes 1920x1080w" null))
    (:`NewEnumerator2`
      (`KismetSystemLibrary.ExecuteConsoleCommand` "r.setRes 1280x720w" null))
    (:`NewEnumerator3`
      (`KismetSystemLibrary.ExecuteConsoleCommand` "r.setRes 960x540w" null)))
  (return false))

(fn `UserConstructionScript`)