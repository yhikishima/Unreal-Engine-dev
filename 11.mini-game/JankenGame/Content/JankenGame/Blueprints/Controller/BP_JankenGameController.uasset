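; Actor that runs a janken (rock-paper-scissors) match, wiring up game, result and Space-opened menu widgets.
; Each selection faces a random enemy hand through JudgeJanken, storing wins and losses in BP_GameState and replaying draws uncounted.
; At JankenCountMax rounds, it compares win counts, plays the outcome sound and shows results.
; Widget events handle continue, resume, quit and delayed return to Title behind a loading screen.
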(event `OnClickedFromResultToTitle`
  (bind _returnvalue (`|CreateWidget` "/Game/JankenGame/Blueprints/UMG/WBP_Loading.WBP_Loading_C"))
  (`UserWidget.AddToViewport` _returnvalue 0)
  (`KismetSystemLibrary.Delay` 2.0)
  (`GameplayStatics.OpenLevel` "Title"))

(event `OnClickedContinue`
  ;[1 1 1] 変数の初期化
  (`/Game/JankenGame/Core/BP_GameState.Initialize` (`self.GameState`))
  (`self.OnCallJanken`)
  (`Widget.RemoveFromParent` (`self.WidgetGameResult`)))

(event `self.ReceiveBeginPlay`
  (`|ExecutionSequence`
    (:`then_0`
      ;[1 1 1] GameStateをBP_GameStateにキャストして変数に設定
      (bind _asbp_game_state (cast `/Game/JankenGame/Core/BP_GameState` (`GameplayStatics.GetGameState`))
        (:`then`
          (set `self.GameState` _asbp_game_state))
        (:`CastFailed`
          (`KismetSystemLibrary.PrintString` "Cast Failed"))))
    (:`then_1`
      ;[1 1 1] じゃんけんの選択画面を表示する
      (bind _returnvalue (`|CreateWidget` "/Game/JankenGame/Blueprints/UMG/WBP_Game.WBP_Game_C"))
      (add `/Game/JankenGame/Blueprints/UMG/WBP_Game.OnHoverdJanken` _returnvalue (delegate `OnHoverdJanken`))
      (add `/Game/JankenGame/Blueprints/UMG/WBP_Game.OnSelectJanken` _returnvalue (delegate `OnSelectJankenGu`))
      (`UserWidget.AddToViewport` _returnvalue 0))
    (:`then_2`
      (bind _returnvalue_2 (`|CreateWidget` "/Game/JankenGame/Blueprints/UMG/WBP_GameResult.WBP_GameResult_C"))
      (add `/Game/JankenGame/Blueprints/UMG/WBP_GameResult.OnClickedContinue` _returnvalue_2 (delegate `OnClickedContinue`))
      (add `/Game/JankenGame/Blueprints/UMG/WBP_GameResult.OnClickedFromResultToTile` _returnvalue_2 (delegate `OnClickedFromResultToTitle`))
      (set `self.WidgetGameResult` _returnvalue_2))
    (:`then_3`
      ;[1 1 1] キーボード入力を有効にする
      (`self.EnableInput` (`GameplayStatics.GetPlayerController` 0)))
    (:`then_4`
      (`GameplayStatics.PlaySound2D` "/Game/JankenGame/Audio/BGM/A_Janken_Game_Cue.A_Janken_Game_Cue" 1.0 1.0 0.0 null null)
      (`self.OnCallJanken`))))

(event `self.ReceiveTick`
  (params (DeltaSeconds :type "Float (single-precision)"))
  (set `PlayerController.bShowMouseCursor` true (`GameplayStatics.GetPlayerController` 0)))

(event `OnSelectJankenGu`
  (params (SelectJanken :type "/Game/JankenGame/Blueprints/Enums/EJanken Enum" :default "NewEnumerator0"))
  (bind _gamestate (`self.GameState`))
  (bind _gamestate_2 (`self.GameState`))
  (bind _gamestate_3 (`self.GameState`))
  (bind _gamestate_4 (`self.GameState`))
  (bind _gamestate_5 (`self.GameState`))
  (bind _widgetgameresult (`self.WidgetGameResult`))
  (bind _playerjanken (`/Game/JankenGame/Core/BP_GameState.PlayerJanken` _gamestate_4))
  (bind _enemyjanken (`/Game/JankenGame/Core/BP_GameState.EnemyJanken` _gamestate_4))
  (bind _jankenresults (`/Game/JankenGame/Core/BP_GameState.JankenResults` _gamestate_4))
  (set `/Game/JankenGame/Core/BP_GameState.PlayerJanken` SelectJanken (`self.GameState`))
  (bind _result (`self.PlayEnemyJanken`))
  (set `/Game/JankenGame/Core/BP_GameState.EnemyJanken` _result _gamestate_3)
  (bind _result_2 (`self.JudgeJanken` (`/Game/JankenGame/Core/BP_GameState.PlayerJanken` _gamestate_3) (`/Game/JankenGame/Core/BP_GameState.EnemyJanken` _gamestate_3)))
  (switch `/Game/JankenGame/Blueprints/Enums/EJankenResult` _result_2
    (:`NewEnumerator0`
      (`KismetArrayLibrary.Array_Add` _jankenresults (make `/Game/JankenGame/Blueprints/Structs/FJankenResult` true _playerjanken _enemyjanken))
      (`/Engine/EditorBlueprintResources/StandardMacros.IncrementInt` (`/Game/JankenGame/Core/BP_GameState.PlayerWinCount` (`self.GameState`))
        (:`  `
          ;[1 1 1] じゃんけんの勝敗がJankenCountMax(5)を越えていないか確認
          (if (< (`KismetArrayLibrary.Array_Length` (`/Game/JankenGame/Core/BP_GameState.JankenResults` _gamestate)) (`/Game/JankenGame/Core/BP_GameState.JankenCountMax` _gamestate)) :!label _label
            (`self.OnCallJanken`)
            (else
              ;[1 1 1] 結果画面の表示
              (set `/Game/JankenGame/Core/BP_GameState.CallJankenStr` "" (`self.GameState`))
              (`/Game/JankenGame/Blueprints/UMG/WBP_GameResult.SetJankenResults` _widgetgameresult)
              (`UserWidget.AddToViewport` _widgetgameresult 0)
              ;[1 1 1] 勝敗を判定
              (`/Engine/EditorBlueprintResources/StandardMacros.CompareInt` (`/Game/JankenGame/Core/BP_GameState.EnemyWinCount` _gamestate_5) (`/Game/JankenGame/Core/BP_GameState.PlayerWinCount` _gamestate_5)
                (:`>`
                  (set `/Game/JankenGame/Core/BP_GameState.GameResult` "NewEnumerator1" _gamestate_2)
                  (`GameplayStatics.PlaySound2D` "/Game/JankenGame/Audio/SE/A_Lose.A_Lose" 1.0 1.0 0.0 null null))
                (:`==`
                  (set `/Game/JankenGame/Core/BP_GameState.GameResult` "NewEnumerator2" _gamestate_2)
                  (`GameplayStatics.PlaySound2D` "/Game/JankenGame/Audio/SE/A_Draw.A_Draw" 1.0 1.0 0.0 null null))
                (:`<`
                  (set `/Game/JankenGame/Core/BP_GameState.GameResult` "NewEnumerator0" _gamestate_2)
                  (`GameplayStatics.PlaySound2D` "/Game/JankenGame/Audio/SE/A_Win.A_Win" 1.0 1.0 0.0 null null)))
              ;[1 1 1] 5回分の勝敗を出力する
              (for _array_element (`/Game/JankenGame/Core/BP_GameState.JankenResults` (`self.GameState`))
                _))))))
    (:`NewEnumerator1`
      (`KismetArrayLibrary.Array_Add` _jankenresults (make `/Game/JankenGame/Blueprints/Structs/FJankenResult` false _playerjanken _enemyjanken))
      (`/Engine/EditorBlueprintResources/StandardMacros.IncrementInt` (`/Game/JankenGame/Core/BP_GameState.EnemyWinCount` (`self.GameState`))
        (:`  `
          (goto _label))))
    (:`NewEnumerator2`
      (`self.OnCallDraw`))))

(event `OnHoverdJanken`
  (params (HoverdJanken :type "/Game/JankenGame/Blueprints/Enums/EJanken Enum" :default "NewEnumerator0"))
  (set `/Game/JankenGame/Core/BP_GameState.PlayerJanken` HoverdJanken (`self.GameState`)))

(event `self.ReceiveActorBeginOverlap`
  (params (OtherActor :type "Actor Object Reference")))

(event `OnCallJanken`
  ;[1 1 1] じゃんけんを出力
  (set `/Game/JankenGame/Core/BP_GameState.CallJankenStr` "じゃんけん" (`self.GameState`))
  (`GameplayStatics.PlaySound2D` "/Game/JankenGame/Audio/SE/A_Janken.A_Janken" 1.0 1.0 0.0 null null))

(event `Key|SpaceBar`
  (params (Key :type "Key Structure"))
  ;[1 1 1] Menu表示
  (:`Pressed`
    (`/Engine/EditorBlueprintResources/StandardMacros.DoOnce` false :!label _label_2
      (:`Completed`
        (bind _returnvalue (`|CreateWidget` "/Game/JankenGame/Blueprints/UMG/WBP_Menu.WBP_Menu_C"))
        (bind _output_get (set `self.WidgetMenu` _returnvalue))
        (add `/Game/JankenGame/Blueprints/UMG/WBP_Menu.OnClickedResume` _output_get (delegate `OnClickedResume`))
        (add `/Game/JankenGame/Blueprints/UMG/WBP_Menu.OnClickedFromMenuToTile` _output_get (delegate `OnClickedFromMenuToTile`))
        (add `/Game/JankenGame/Blueprints/UMG/WBP_Menu.OnClickedGameExit` _output_get (delegate `OnClickedGameExit`))
        (`UserWidget.AddToViewport` _output_get 0)))))

(event `OnCallDraw`
  ;[1 1 1] あいこの出力
  (set `/Game/JankenGame/Core/BP_GameState.CallJankenStr` "あいこ" (`self.GameState`))
  (`GameplayStatics.PlaySound2D` "/Game/JankenGame/Audio/SE/A_AikoDe.A_AikoDe" 1.0 1.0 0.0 null null))

(event `OnClickedResume`
  ;[1 1 1] 再開ボタンの処理
  (`Widget.RemoveFromParent` (`self.WidgetMenu`))
  (goto _label_2 :!via `Reset`))

(event `OnClickedFromMenuToTile`
  ;[1 1 1] Menuからタイトルへ
  (bind _returnvalue (`|CreateWidget` "/Game/JankenGame/Blueprints/UMG/WBP_Loading.WBP_Loading_C"))
  (`UserWidget.AddToViewport` _returnvalue 0)
  (`KismetSystemLibrary.Delay` 2.0)
  (`GameplayStatics.OpenLevel` "Title"))

(event `OnClickedGameExit`
  (`KismetSystemLibrary.QuitGame` null "Quit"))

(fn `JudgeJanken`
  (params (ArgPlayerJanken :type "/Game/JankenGame/Blueprints/Enums/EJanken Enum" :default "NewEnumerator0") (ArgEnemyJanken :type "/Game/JankenGame/Blueprints/Enums/EJanken Enum" :default "NewEnumerator0"))
  (returns (Result :type "/Game/JankenGame/Blueprints/Enums/EJankenResult Enum"))
  (switch `/Game/JankenGame/Blueprints/Enums/EJanken` ArgPlayerJanken
    (:`NewEnumerator0`
      (switch `/Game/JankenGame/Blueprints/Enums/EJanken` ArgEnemyJanken ; グー（Gu） vs
        (:`NewEnumerator0`
          (return "NewEnumerator2"))
        (:`NewEnumerator1`
          (return "NewEnumerator0"))
        (:`NewEnumerator2`
          (return "NewEnumerator1"))))
    (:`NewEnumerator1`
      (switch `/Game/JankenGame/Blueprints/Enums/EJanken` ArgEnemyJanken ; チョキ（Choki） vs
        (:`NewEnumerator0`
          (return "NewEnumerator1"))
        (:`NewEnumerator1`
          (return "NewEnumerator2"))
        (:`NewEnumerator2`
          (return "NewEnumerator0"))))
    (:`NewEnumerator2`
      (switch `/Game/JankenGame/Blueprints/Enums/EJanken` ArgEnemyJanken ; パー（Pa） vs
        (:`NewEnumerator0`
          (return "NewEnumerator0"))
        (:`NewEnumerator1`
          (return "NewEnumerator1"))
        (:`NewEnumerator2`
          (return "NewEnumerator2"))))))

(fn `PlayEnemyJanken`
  (returns (Result :type "/Game/JankenGame/Blueprints/Enums/EJanken Enum"))
  (switch `int` (`KismetMathLibrary.RandomInteger` 3)
    (:`0`
      (return "NewEnumerator0"))
    (:`1`
      (return "NewEnumerator1"))
    (:`2`
      (return "NewEnumerator2"))))

(fn `UserConstructionScript`)