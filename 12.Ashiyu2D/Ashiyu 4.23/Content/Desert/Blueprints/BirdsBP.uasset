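; BirdsBP is a Paper2D bird flock that flies horizontally across the scene and destroys itself after a minute.
; The construction script picks a random left or right direction, then adds five mirrored-to-match flipbook birds at random points inside a box, each with a random play rate.
; On BeginPlay, ProjectileMovement moves the whole flock along local X at a random speed in that direction.
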(event `SkySpeed`
  (`ProjectileMovementComponent.SetVelocityInLocalSpace` (`self.ProjectileMovement`) (`KismetMathLibrary.MakeVector` (* (`KismetMathLibrary.RandomFloatInRange` 100.0 200.0) (select `bool` (`self.Backward`) :`false` 1.0 :`true` -1.0 :!type "Float (single-precision)"))) :!label _label)
  (`KismetSystemLibrary.Delay` 60.0)
  (`self.K2_DestroyActor`))

(event `self.ReceiveBeginPlay`
  (goto _label))

(fn `BirdsAdd`
  (bind _box (`self.Box`))
  (bind _returnvalue (`AddComponent|NODE_AddPaperFlipbookComponent-1` :`RelativeTransform` (`KismetMathLibrary.MakeTransform` (`KismetMathLibrary.RandomPointInBoundingBox` (`SceneComponent.RelativeLocation` _box) (`BoxComponent.BoxExtent` _box)) (struct) (`KismetMathLibrary.MakeVector` (select `bool` (`self.Backward`) :`false` -1.0 :`true` 1.0 :!type "Float (single-precision)") 1.0 1.0))))
  (`PaperFlipbookComponent.SetPlayRate` _returnvalue (`KismetMathLibrary.RandomFloatInRange` 0.5 1.5))
  (`KismetArrayLibrary.Array_Add` (`self.BirdsArr`) _returnvalue))

(fn `DirectionRandomizer`
  (bind _arrow (`self.Arrow`))
  (set `self.Backward` (`KismetMathLibrary.RandomBool`))
  (if (`self.Backward`)
    (`SceneComponent.SetRelativeScale3D` _arrow (-1.0 1.0 1.0))
    (else
      (`SceneComponent.SetRelativeScale3D` _arrow (1.0 1.0 1.0)))))

(fn `UserConstructionScript`
  (`self.DirectionRandomizer`)
  (for _ (range 1 6)
    (`self.BirdsAdd`)))