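; BirdSpawnerBP spawns flocks of birds that fly horizontally across the sky around the player.
; A looping SpawnTime timer creates a BirdsBP left or right of the player, offset by the player-to-camera distance.
; World height is random, derived from viewport pixel height.
; Each flock gets a random speed toward the player's side, and its BirdsArr elements are mirrored on X to match the flight direction.
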(event `SpawnSky`
  (bind _returnvalue (`self.K2_GetActorLocation` (`GameplayStatics.GetPlayerPawn` 0)))
  (bind (_x _y) (`KismetMathLibrary.BreakVector2D` (`WidgetLayoutLibrary.GetViewportSize`)))
  (bind _x_2 (.x _returnvalue))
  (bind _returnvalue_2 (`KismetMathLibrary.VSize` (- _returnvalue (`self.K2_GetActorLocation` (`GameplayStatics.GetPlayerCameraManager` 0)))))
  (bind _returnvalue_3 (`|SpawnActorFromClass` "/Game/Desert/Blueprints/BirdsBP.BirdsBP_C" (`KismetMathLibrary.MakeTransform` (`KismetMathLibrary.MakeVector` (select `int` (`KismetMathLibrary.RandomIntegerInRange` 0 1) :`0` (- _x_2 _returnvalue_2) :`1` (+ _x_2 _returnvalue_2)) (.y _returnvalue) (`KismetMathLibrary.RandomFloatInRange` (/ _y 2.0) _y))) "Undefined" "OverrideRootScale" null null))
  (bind _returnvalue_x (`KismetMathLibrary.BreakVector` (`self.K2_GetActorLocation` _returnvalue_3)))
  (bind _returnvalue_4 (< _returnvalue_x _x_2))
  (`ProjectileMovementComponent.SetVelocityInLocalSpace` (`/Game/Desert/Blueprints/BirdsBP.ProjectileMovement` _returnvalue_3) (`KismetMathLibrary.MakeVector` (* (`KismetMathLibrary.RandomFloatInRange` 100.0 200.0) (select `bool` _returnvalue_4 :`false` -1.0 :`true` 1.0 :!type "Float (single-precision)"))))
  (for _array_element (`/Game/Desert/Blueprints/BirdsBP.BirdsArr` _returnvalue_3)
    (`SceneComponent.SetRelativeScale3D` _array_element (`KismetMathLibrary.MakeVector` (select `bool` _returnvalue_4 :`false` 1.0 :`true` -1.0 :!type "Float (single-precision)") 1.0 1.0))))

(event `self.ReceiveBeginPlay`
  (`KismetSystemLibrary.K2_SetTimerDelegate` (delegate `SpawnSky`) (`self.SpawnTime`) true))

(fn `UserConstructionScript`)