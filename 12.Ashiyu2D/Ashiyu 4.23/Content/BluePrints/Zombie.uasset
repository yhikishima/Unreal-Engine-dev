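; Player-controlled 2D flipbook Zombie character that walks along the X axis with A/D and triggers attack, spawn and death with mouse and keys.
; Tick applies movement and runs a priority-based state function that picks the flipbook and its looping from state flags.
; Finished one-shot flipbooks clear the attack and spawn flags.
; Death disables input, blinks the sprite via a timeline, then possesses a new Zombie at PlayerStart and destroys this one.
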(event `Key|A`
  (params (Key :type "Key Structure"))
  ;[1 1 1] A key held
  (:`Pressed`
    (set `self.A_Held` true))
  (:`Released`
    (set `self.A_Held` false)))

(event `Key|D`
  (params (Key :type "Key Structure"))
  ;[1 1 1] D key held
  (:`Pressed`
    (set `self.D_Held` true))
  (:`Released`
    (set `self.D_Held` false)))

(event `Add Movement`
  (params (ScaleValue :type "Float (double-precision)"))
  ;[1 1 1] Movement
  (`self.AddMovementInput` (1.0 0.0 0.0) ScaleValue)
  (`/Engine/EditorBlueprintResources/StandardMacros.CompareFloat` ScaleValue
    (:`>`
      (`Controller.SetControlRotation` (`self.GetController`) (`KismetMathLibrary.MakeRotator` 0.0)))
    (:`<`
      (`Controller.SetControlRotation` (`self.GetController`) (`KismetMathLibrary.MakeRotator` 0.0 0.0 180.0)))))

(event `self.ReceiveTick`
  (params (DeltaSeconds :type "Float (single-precision)"))
  (`self.UpdateAnimation`)
  (if (not (`self.isDead`))
    (`|ExecutionSequence`
      (:`then_0`
        ;[1 1 1] Add movement left
        (if (`self.A_Held`)
          (`self.Add Movement` -1.0)))
      (:`then_1`
        ;[1 1 1] Add movement right
        (if (`self.D_Held`)
          (`self.Add Movement` 1.0))))))

(event `UpdateAnimation`
  ;[1 1 1] Update Animation
  (set `self.isMoving` (> (`KismetMathLibrary.Abs` (.x (`self.GetVelocity`))) 0.0))
  (bind _outputanimation (`self.AnimationStatesMachine`))
  (`PaperFlipbookComponent.SetFlipbook` (`self.Sprite`) _outputanimation))

(event `self.Sprite.OnFinishedPlaying`
  ;[1 1 1] On finished playing flipbook
  (set `self.isAttacking` false)
  (set `self.isSpawning` false))

(event `Key|LeftMouseButton`
  (params (Key :type "Key Structure"))
  ;[1 1 1] Attack
  (:`Pressed`
    (set `self.isAttacking` true)))

(event `Key|Q`
  (params (Key :type "Key Structure"))
  ;[1 1 1] Spawn
  (:`Pressed`
    (set `self.isSpawning` true)))

(event `Key|E`
  (params (Key :type "Key Structure"))
  ;[1 1 1] Death
  (:`Pressed`
    (set `self.isDead` true)
    (`self.DisableInput` (`GameplayStatics.GetPlayerController` 0))
    (`KismetSystemLibrary.Delay` 1.5) ; Let death animation play before blinking
    (bind (_direction _alpha) (`Timeline|Sprite Blinker` :!via `PlayFromStart`)
      (:`Update`
        (if (> _alpha (* (`KismetMathLibrary.Conv_IntToDouble` (`self.CurrentBlink`)) (/ 1.0 (`KismetMathLibrary.Conv_IntToDouble` (`self.DeathBlinks`)))))
          (`/Engine/EditorBlueprintResources/StandardMacros.IncrementInt` (`self.CurrentBlink`)
            (:`  `
              (`self.Blink Sprite`)))))
      (:`Finished`
        (`SceneComponent.SetVisibility` (`self.Sprite`) false false)
        (`self.SetActorEnableCollision` false)
        (bind _outactors (`GameplayStatics.GetAllActorsOfClass` "/Script/Engine.PlayerStart")) ; Get player start location
        (bind _returnvalue (`|SpawnActorFromClass` "Zombie_C" (`KismetMathLibrary.MakeTransform` (`self.K2_GetActorLocation` (`|GetArrayItem` _outactors))) "Undefined" "OverrideRootScale" (`GameplayStatics.GetPlayerController` 0) null))
        (`Controller.Possess` (`GameplayStatics.GetPlayerController` 0) _returnvalue)
        (`self.K2_DestroyActor`) ; Destroy old character
      ))))

(event `Blink Sprite`
  ;[1 1 1] Blink Sprite
  (`SceneComponent.SetVisibility` (`self.Sprite`) false false)
  (`KismetSystemLibrary.Delay` 0.1)
  (`SceneComponent.SetVisibility` (`self.Sprite`) true false))

(fn `AnimationStatesMachine`
  (returns (outputAnimation :type "PaperFlipbook Object Reference"))
  (locals (AnimationState :type "/Game/BluePrints/ZombieAnimationStates Enum") (isPlayFromStart :type Boolean))
  ;[1 1 1] Check conditions
  (if (`self.isDead`)
    ;[1 1 1] Set Animation state
    (set `local.AnimationState` "NewEnumerator3")
    ;[1 1 1] Call setLooping function
    (`self.setLooping` false :!label _label)
    (elif (`self.isSpawning`)
      (set `local.AnimationState` "NewEnumerator4")
      (goto _label)
      (elif (`self.isAttacking`)
        (set `local.AnimationState` "NewEnumerator2")
        (goto _label)
        (else
          (if (`self.isMoving`)
            (set `local.AnimationState` "NewEnumerator1")
            (else
              (set `local.AnimationState` "NewEnumerator0")))
          (`self.setLooping` true)))))
  ;[1 1 1] Return desired animation
  (return (select `/Game/BluePrints/ZombieAnimationStates` (`local.AnimationState`) :`NewEnumerator0` (`self.IdleFlipbook`) :`NewEnumerator1` (`self.WalkFlipbook`) :`NewEnumerator2` (`self.AttackFlipbook`) :`NewEnumerator3` (`self.DeathFlipbook`) :`NewEnumerator4` (`self.SpawnFlipbook`))))

(fn `setLooping`
  (params (shouldLoop :type Boolean))
  ;[1 1 1] Set if the animation should loop or not
  (`PaperFlipbookComponent.SetLooping` (`self.Sprite`) shouldLoop)
  ;[1 1 1] Restart flipbook if it stops playing
  (if (not (`PaperFlipbookComponent.IsPlaying` (`self.Sprite`)))
    (`PaperFlipbookComponent.Play` (`self.Sprite`))))

(fn `UserConstructionScript`)