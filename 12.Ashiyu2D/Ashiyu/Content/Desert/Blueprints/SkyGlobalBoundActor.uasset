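; Desert sky actor that fills a box volume with randomly placed cloud sprites and seeds sky and cloud actors at runtime.
; The construction script sizes and offsets Box from SizeBox (Y not halved), then adds CloudCount Paper sprite components at random points inside, using random CloudVariationArr sprites.
; On BeginPlay, it spawns both a SkySpawnerBP and a CloudsBP at the world location of every descendant component of the root.
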(event `self.ReceiveBeginPlay`
  (for _array_element (`SceneComponent.GetChildrenComponents` (`self.DefaultSceneRoot`) true)
    (bind _returnvalue (`SceneComponent.K2_GetComponentLocation` _array_element))
    (`|SpawnActorFromClass` "/Game/Desert/Blueprints/SkySpawnerBP.SkySpawnerBP_C" (`KismetMathLibrary.MakeTransform` _returnvalue) "Undefined" "OverrideRootScale" null null)
    (`|SpawnActorFromClass` "/Game/Desert/Blueprints/CloudsBP.CloudsBP_C" (`KismetMathLibrary.MakeTransform` _returnvalue) "Undefined" "OverrideRootScale" null null)))

(fn `UserConstructionScript`
  (bind _box (`self.Box`))
  (bind _cloudvariationarr (`self.CloudVariationArr`))
  (bind _returnvalue (`KismetMathLibrary.MakeVector` (/ (.x (`self.SizeBox`)) 2.0) (.y (`self.SizeBox`)) (/ (.z (`self.SizeBox`)) 2.0)))
  (`BoxComponent.SetBoxExtent` (`self.Box`) _returnvalue false)
  (`SceneComponent.K2_SetRelativeLocation` (`self.Box`) _returnvalue false false)
  (for _ (range 1 (+ (`self.CloudCount`) 1))
    (if (not false)
      (bind _returnvalue_2 (`AddComponent|NODE_AddPaperSpriteComponent-0` :`RelativeTransform` (`KismetMathLibrary.MakeTransform` (`KismetMathLibrary.RandomPointInBoundingBox` (`SceneComponent.RelativeLocation` _box) (`BoxComponent.BoxExtent` _box)) (struct) (1.0 1.0 1.0))))
      (`PaperSpriteComponent.SetSprite` _returnvalue_2 (`|GetArrayItem` _cloudvariationarr (`KismetMathLibrary.RandomInteger` (`KismetArrayLibrary.Array_Length` _cloudvariationarr)))))))