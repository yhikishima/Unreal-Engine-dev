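; TrainBP is a 2D sprite train that travels left or right along X at a random speed.
; The construction script appends a random number of sprite cars behind the main sprite, sorted at a lower translucent priority.
; The Backward flag mirrors the sprites, arrow and particle effect, and sets DirectionX.
; On BeginPlay, DirectionX signs a random local velocity given to the ProjectileMovement component.
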(event `self.ReceiveBeginPlay`
  (`ProjectileMovementComponent.SetVelocityInLocalSpace` (`self.ProjectileMovement`) (`KismetMathLibrary.MakeVector` (* (`KismetMathLibrary.RandomFloatInRange` 100.0 200.0) (`self.DirectionX`)))))

(fn `UserConstructionScript`
  (bind _arrow (`self.Arrow`))
  (bind _backward (`self.Backward`))
  ;[1 1 1] Left or Right direction
  (`SceneComponent.K2_SetRelativeTransform` (`self.ParticleSystem`) (`KismetMathLibrary.MakeTransform` (`KismetMathLibrary.MakeVector` (select `bool` _backward :`false` 15.0 :`true` -15.0 :!type "Float (single-precision)") 0.0 25.0) (struct) (`KismetMathLibrary.MakeVector` (select `bool` _backward :`false` -0.1 :`true` 0.1 :!type "Float (single-precision)") 0.1 0.1)) false false)
  (for _index (range 1 (+ (`KismetMathLibrary.RandomIntegerInRange` 3 9) 1))
    (bind _returnvalue (`AddComponent|NODE_AddPaperSpriteComponent-0` :`RelativeTransform` (`KismetMathLibrary.MakeTransform` (`KismetMathLibrary.MakeVector` (* _index (select `bool` _backward :`false` -71.0 :`true` 71.0 :!type "Float (single-precision)")) 0.0 0.0))))
    (`PrimitiveComponent.SetTranslucentSortPriority` _returnvalue -5)
    (if (`self.Backward`)
      (`SceneComponent.SetRelativeScale3D` _arrow (-1.0 1.0 1.0))
      (`SceneComponent.SetRelativeScale3D` (`self.Main`) (-1.0 1.0 1.0))
      (`SceneComponent.SetRelativeScale3D` _returnvalue (-1.0 1.0 1.0))
      (set `self.DirectionX` -1.0)
      (else
        (`SceneComponent.SetRelativeScale3D` _arrow (1.0 1.0 1.0))
        (`SceneComponent.SetRelativeScale3D` (`self.Main`) (1.0 1.0 1.0))
        (`SceneComponent.SetRelativeScale3D` _returnvalue (1.0 1.0 1.0))
        (set `self.DirectionX` 1.0)))))