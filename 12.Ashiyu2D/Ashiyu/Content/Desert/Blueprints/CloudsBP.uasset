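; CloudsBP is a drifting cloud actor for the Desert content, shown as a Paper2D sprite.
; Its construction script picks a random sprite and a left or right X direction, flipping an arrow component to match.
; From BeginPlay, a looping timer periodically re-randomizes the ProjectileMovement speed along that direction.
; An opacity timeline meant to fade and destroy the cloud is present but never runs.
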(event `SkySpeed`
  (`ProjectileMovementComponent.SetVelocityInLocalSpace` (`self.ProjectileMovement`) (`KismetMathLibrary.MakeVector` (* (`KismetMathLibrary.RandomFloatInRange` 10.0 30.0) (`self.DirectionX`))) :!label _label)
  (`KismetSystemLibrary.K2_SetTimerDelegate` (delegate `SkySpeed`) 3.0 true))

(event `self.ReceiveBeginPlay`
  (goto _label))

(fn `RandomizedCloud`
  (bind _arrow (`self.Arrow`))
  (bind _skyarr (`self.SkyArr`))
  (set `self.Backward` (`KismetMathLibrary.RandomBool`))
  (`PaperSpriteComponent.SetSprite` (`self.PaperSprite`) (`|GetArrayItem` _skyarr (`KismetMathLibrary.RandomInteger` (`KismetArrayLibrary.Array_Length` _skyarr))))
  (if (`self.Backward`)
    (`SceneComponent.SetRelativeScale3D` _arrow (-1.0 1.0 1.0))
    (set `self.DirectionX` -1.0)
    (else
      (`SceneComponent.SetRelativeScale3D` _arrow (1.0 1.0 1.0))
      (set `self.DirectionX` 1.0))))

(fn `UserConstructionScript`
  (`self.RandomizedCloud`))