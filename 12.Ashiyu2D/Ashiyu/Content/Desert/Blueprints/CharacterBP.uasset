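; Paper2D side-scroller player character with run, jump, slide and shoot states, plus a camera height set from the viewport aspect ratio at start.
; Input and Slide/Shoot events set AnimState, which Tick uses to pick the flipbook, with falling always showing Jump.
; Slide replays the captured move input through a timeline, while Shoot is only a brief movement-blocking pose.
; Tick also line-traces to place the shadow and yaws the controller to face travel direction.
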(event `self.ReceiveBeginPlay`
  (bind (_returnvalue_x _returnvalue_y) (`KismetMathLibrary.BreakVector2D` (`WidgetLayoutLibrary.GetViewportSize`)))
  ;[1 1 1] Set camers height 4:3 / 16:9
  (`ActorComponent.SetIsReplicated` (`self.Sprite`) true)
  (set `PlayerController.bShowMouseCursor` true (`GameplayStatics.GetPlayerController` 0))
  (`SceneComponent.K2_SetRelativeLocation` (`self.CameraBoom`) (`KismetMathLibrary.MakeVector` 0.0 0.0 (select `bool` (> (/ _returnvalue_x _returnvalue_y) 1.5) :`false` 380.0 :`true` 280.0 :!type "Float (single-precision)")) false false))

(event `InputAction|Jump`
  (params (Key :type "Key Structure"))
  ;[1 1 1] Jump / Slide / Fire
  (:`Pressed`
    (if (not (`|EnumEquality` (`self.AnimState`) "NewEnumerator3"))
      (`self.Jump`)
      (set `self.AnimState` "NewEnumerator2")))
  (:`Released`
    (`self.StopJumping`)
    (set `self.AnimState` "NewEnumerator0")))

(event `InputAxis|MoveRight`
  (params (AxisValue :type "Float (single-precision)"))
  (bind _animstate (`self.AnimState`))
  ;[1 1 1] Handle movement
  (if (not (or (`|EnumEquality` _animstate "NewEnumerator3") (`|EnumEquality` _animstate "NewEnumerator4")))
    (if (> AxisValue 0.0)
      (set `self.bisMovingRight` true)
      (elif (< AxisValue 0.0)
        (set `self.bisMovingRight` false)))
    (`self.AddMovementInput` (1.0 0.0 0.0) AxisValue)))

(event `UpdateAnimation`
  (bind _sprite (`self.Sprite`))
  ;[1 1 1] Jump / Slide / Fire
  (if (`NavMovementComponent.IsFalling` (`self.CharacterMovement`))
    (`PaperFlipbookComponent.SetFlipbook` (`self.Sprite`) "/Game/Desert/Sprites/CowGirl/Frames/Jump.Jump")
    (else
      (switch `/Game/Desert/Blueprints/AnimState` (`self.AnimState`)
        (:`NewEnumerator0`
          (`PaperFlipbookComponent.SetFlipbook` _sprite (select `bool` (> (`KismetMathLibrary.VSize` (`self.GetVelocity`)) 0.0) :`false` "/Game/Desert/Sprites/CowGirl/Frames/Idle.Idle" :`true` "/Game/Desert/Sprites/CowGirl/Frames/Run.Run" :!type "PaperFlipbook Object Reference") :!label _label))
        (:`NewEnumerator1`
          (goto _label))
        (:`NewEnumerator2`
          (`PaperFlipbookComponent.SetFlipbook` _sprite "/Game/Desert/Sprites/CowGirl/Frames/Jump.Jump"))
        (:`NewEnumerator3`
          (`PaperFlipbookComponent.SetFlipbook` _sprite "/Game/Desert/Sprites/CowGirl/Frames/Slide.Slide")
          (`/Engine/EditorBlueprintResources/StandardMacros.DoOnce` false :!label _label_2
            (:`Completed`
              (bind (_direction _newtrack_1) (`Timeline|Timeline_0` :!via `PlayFromStart`)
                (:`Update`
                  (`self.AddMovementInput` (1.0 0.0 0.0) (* _newtrack_1 (`self.TempVelocity`))))
                (:`Finished`
                  (set `self.AnimState` "NewEnumerator0")
                  (goto _label_2 :!via `Reset`))))))
        (:`NewEnumerator4`
          (`PaperFlipbookComponent.SetFlipbook` _sprite "/Game/Desert/Sprites/CowGirl/Frames/Shoot.Shoot")
          (`self.AddMovementInput` (0.0 0.0 0.0) 0.0))))))

(event `Slide`
  ;[1 1 1] Jump / Slide / Fire
  (set `self.AnimState` "NewEnumerator3")
  (set `self.TempVelocity` (`self.GetInputAxisValue`)))

(event `Shoot`
  ;[1 1 1] Jump / Slide / Fire
  (if (not (`|EnumEquality` (`self.AnimState`) "NewEnumerator3"))
    (set `self.AnimState` "NewEnumerator4")
    (`KismetSystemLibrary.Delay` 0.3)
    (set `self.AnimState` "NewEnumerator0")))

(event `self.ReceiveTick`
  (params (DeltaSeconds :type "Float (single-precision)"))
  (bind _arrow1 (`self.Arrow1`))
  (bind _returnvalue (`SceneComponent.K2_GetComponentLocation` _arrow1))
  ;[1 1 1] Tick - Updates animation
  (`|ExecutionSequence`
    (:`then_0`
      ;[1 1 1] Shadow under character
      (bind _outhit (`KismetSystemLibrary.LineTraceSingle` _returnvalue (+ _returnvalue (* (`KismetMathLibrary.GetForwardVector` (`SceneComponent.K2_GetComponentRotation` _arrow1)) 1000.0)) "TraceTypeQuery1"))
      (`SceneComponent.K2_SetWorldLocation` (`self.Shadow`) (`.Location` (`GameplayStatics.BreakHitResult` _outhit)) false false))
    (:`then_1`
      (`self.UpdateAnimation`)
      (`/Engine/EditorBlueprintResources/StandardMacros.CompareFloat` (.x (`MovementComponent.Velocity` (`self.GetMovementComponent`)))
        (:`>`
          (`Controller.SetControlRotation` (`self.GetController`) (`KismetMathLibrary.MakeRotator` 0.0) :!label _label_3))
        (:`==`
          (if (`self.bisMovingRight`)
            (goto _label_3)
            (else
              (`Controller.SetControlRotation` (`self.GetController`) (`KismetMathLibrary.MakeRotator` 0.0 0.0 180.0) :!label _label_4))))
        (:`<`
          (goto _label_4))))))

(fn `UserConstructionScript`)