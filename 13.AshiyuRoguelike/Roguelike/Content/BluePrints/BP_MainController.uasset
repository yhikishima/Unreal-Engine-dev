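; BP_MainController is a level controller Blueprint that shows the game UI and detects the clear condition.
; BeginPlay creates WBP_UI and adds it to the viewport.
; Tick polls the EnemyBroken array in BP_GameInstance and, once it holds at least four entries, creates and displays WBP_Clear.
; The check has no one-shot guard, so a new clear widget is added every tick while the condition holds.
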(event `self.ReceiveBeginPlay`
  (bind _returnvalue (`|CreateWidget` "/Game/Wbp/WBP_UI.WBP_UI_C"))
  (`UserWidget.AddToViewport` _returnvalue 0))

(event `self.ReceiveTick`
  (params (DeltaSeconds :type "Float (single-precision)"))
  (bind _asbp_game_instance (cast `/Game/BluePrints/BP_GameInstance` (`GameplayStatics.GetGameInstance`)))
  (if (>= (`KismetArrayLibrary.Array_Length` (`/Game/BluePrints/BP_GameInstance.EnemyBroken` _asbp_game_instance)) 4)
    (bind _returnvalue (`|CreateWidget` "/Game/Wbp/WBP_Clear.WBP_Clear_C"))
    (`UserWidget.AddToViewport` _returnvalue 0)))

(fn `UserConstructionScript`)