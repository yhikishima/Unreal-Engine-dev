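; BP_Character is a player character Blueprint with world-axis movement and an idle/run animation flag.
; MoveForward and MoveRight add movement input along fixed world directions, snapping mesh yaw only at full positive or negative input.
; Tick sets IsRun on BP_GameInstance when speed reaches a threshold.
; An enemy-hit handler, commented as game over, only prints a string, and its binding nodes are never executed.
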(event `self.ReceiveBeginPlay`
  ;[1 1 1] アニメーション（idol <=> run）
  (bind _asbp_game_instance (cast `/Game/BluePrints/BP_GameInstance` (`GameplayStatics.GetGameInstance`))))

(event `self.ReceiveTick`
  (params (DeltaSeconds :type "Float (single-precision)"))
  ;[1 1 1] アニメーション（idol <=> run）
  (if (>= (`KismetMathLibrary.VSize` (`self.GetVelocity` (`PawnMovementComponent.GetPawnOwner` (`self.CharacterMovement`)))) 200.0)
    (set `/Game/BluePrints/BP_GameInstance.IsRun` true (stale `self.ReceiveBeginPlay` _asbp_game_instance))
    (else
      (set `/Game/BluePrints/BP_GameInstance.IsRun` false (stale `self.ReceiveBeginPlay` _asbp_game_instance)))))

(event `InputAxis|MoveForward`
  (params (AxisValue :type "Float (single-precision)"))
  (`self.AddMovementInput` (`PawnMovementComponent.GetPawnOwner` (`self.CharacterMovement`)) (1.0 0.0 0.0) AxisValue false)
  (if (== AxisValue 1.0)
    (`SceneComponent.K2_SetWorldRotation` (`self.Mesh`) (struct :`Yaw` -90.0) false false)
    (elif (== AxisValue -1.0)
      (`SceneComponent.K2_SetWorldRotation` (`self.Mesh`) (struct :`Yaw` 90.0) false false))))

(event `InputAxis|MoveRight`
  (params (AxisValue :type "Float (single-precision)"))
  (`self.AddMovementInput` (`PawnMovementComponent.GetPawnOwner` (`self.CharacterMovement`)) (0.0 1.0 90.0) AxisValue false)
  (if (== AxisValue 1.0)
    (`SceneComponent.K2_SetWorldRotation` :`self` (`self.Mesh`))
    (elif (== AxisValue -1.0)
      (`SceneComponent.K2_SetWorldRotation` (`self.Mesh`) (struct :`Yaw` -180.0) false false))))

(event `OnComponentHit_イベント_0`
  (params (HitComponent :type "PrimitiveComponent Object Reference") (OtherActor :type "Actor Object Reference") (OtherComp :type "PrimitiveComponent Object Reference") (NormalImpulse :type "Vector Structure") (Hit :type "HitResult Structure (by ref)"))
  ;[1 1 1] 敵に当たった。GameOver
  (`KismetSystemLibrary.PrintString` "Hello"))

(fn `UserConstructionScript`)